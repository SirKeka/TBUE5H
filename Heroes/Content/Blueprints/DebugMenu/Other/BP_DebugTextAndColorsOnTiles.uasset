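; Debug-menu actor that draws text over walkable BP_Grid tiles, showing tile index, pathfinding costs and discovery sort order as toggled.
; It binds to grid and pathfinding update and clear events, with a retriggerable delay batching full refreshes to clear stale sort data.
; TextRenderActors are spawned on demand, cached per tile index, scaled to the longest entry and destroyed when nothing is shown.
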(event Custom|Event_ReUpdateAllTextsAfterDelay
  (params (Index :type Int%20Point%20Structure))
  ;[0 0 0] Мы обновяем данные на плитках для того чтобы предыдущие данные сортировки были удалены
  (Utilities|FlowControl|RetriggerableDelay 0.1)
  (CallFunction|UpdateTextonAllTiles))

(event EventBeginPlay
  ;[0 0 0] Привязать к сетке Обратный вызов
  (bind _returnvalue (Actor|GetActorOfClass "/Game/Blueprints/Core/Grid/BP_Grid.BP_Grid_C"))
  (bind _output_get (Variables|Default|SetGrid _returnvalue))
  (EventDispatchers|BindEventtoOnTileDataUpdated _output_get (EventDispatchers|CreateEvent :!event Custom|Event_ReUpdateAllTextsAfterDelay))
  (EventDispatchers|BindEventtoOnGridDestroyed _output_get (EventDispatchers|CreateEvent :!event ClearAllTextActor))
  (EventDispatchers|BindEventtoOnPathfindingDataUpdated (Variables|/Game/Blueprints/Core/Grid/BP_Grid.BP_Grid_C|GetGridPathfinding (Variables|Default|GetGrid)) (EventDispatchers|CreateEvent :!event UpdateTextonTile))
  (EventDispatchers|BindEventtoOnPathfindingDataCleared (Variables|/Game/Blueprints/Core/Grid/BP_Grid.BP_Grid_C|GetGridPathfinding (Variables|Default|GetGrid)) (EventDispatchers|CreateEvent :!event UpdateTextonAllTiles)))

(fn ConstructionScript)

(fn GetTextActor
  (params (Index :type Int%20Point%20Structure))
  (bind _output_get (LocalVariables|SetActor (.Value (Utilities|Map|Find (Variables|Default|GetSpawnedTexts) Index)))) ; Актер уже существует?
  (Utilities|IsValid _output_get
    (:Is%20Valid
      (return (LocalVariables|GetActor)))
    (:Is%20Not%20Valid
      (bind _returnvalue (Game|SpawnActorfromClass "/Script/Engine.TextRenderActor" (Math|Transform|MakeTransform "0, 0, 0" "0, 0, 0" "1.000000,1.000000,1.000000") "AlwaysSpawn" 0 0))
      (bind _output_get_2 (LocalVariables|SetActor _returnvalue))
      (Utilities|Map|Add (Variables|Default|GetSpawnedTexts) Index _output_get_2)
      (Actor|Tick|SetActorTickEnabled (LocalVariables|GetActor))
      (Collision|SetActorEnableCollision (LocalVariables|GetActor) false)
      (Rendering|Components|TextRender|SetHorizontalAlignment (Variables|/Script/Engine.TextRenderActor|GetTextRender (LocalVariables|GetActor)) "EHTA_Center")
      (Class|TextRenderComponent|SetVerticalAlignment (Variables|/Script/Engine.TextRenderActor|GetTextRender (LocalVariables|GetActor)) "EVRTA_TextCenter")
      (return (LocalVariables|GetActor)))))

(fn DestroyTextActor
  (params (Index :type Int%20Point%20Structure%20%28by%20ref%29))
  (bind _output_get (LocalVariables|SetActor (.Value (Utilities|Map|Find (Variables|Default|GetSpawnedTexts) Index))))
  (Utilities|IsValid _output_get
    (:Is%20Valid
      (Actor|DestroyActor _output_get)
      (Utilities|Map|Remove (Variables|Default|GetSpawnedTexts) Index))))

(fn ClearAllTextActor
  (bind _values (Utilities|Map|Values (Variables|Default|GetSpawnedTexts)))
  (for _array_element _values
    (Actor|DestroyActor _array_element))
  (Utilities|Map|Clear (Variables|Default|GetSpawnedTexts)))

(fn UpdateTextonTile
  (params (Index :type Int%20Point%20Structure))
  (bind _grid (Variables|Default|GetGrid))
  (bind _grid_2 (Variables|Default|GetGrid))
  (bind _returnvalue (Utilities|String|ToString(Integer) (.x Index)))
  (bind _returnvalue_2 (Utilities|String|ToString(Integer) (.y Index)))
  (bind _gridtiles (Variables|/Game/Blueprints/Core/Grid/BP_Grid.BP_Grid_C|GetGridTiles _grid))
  (bind _gridpathfinding (Variables|/Game/Blueprints/Core/Grid/BP_Grid.BP_Grid_C|GetGridPathfinding _grid_2))
  (bind (_value _returnvalue_3) (Utilities|Map|Find _gridtiles Index))
  (bind _returnvalue_4 (Utilities|String|Append _returnvalue "," _returnvalue_2))
  (bind _discoveredtileindexes (Variables|/Game/Blueprints/Core/Grid/BP_GridPathfinding.BP_GridPathfinding_C|GetDiscoveredTileIndexes _gridpathfinding))
  (bind _discoveredtilesortibgcost (Variables|/Game/Blueprints/Core/Grid/BP_GridPathfinding.BP_GridPathfinding_C|GetDiscoveredTileSortibgCost _gridpathfinding))
  (bind _returnvalue_5 (Utilities|Array|FindItem _discoveredtileindexes Index))
  (bind _returnvalue_6 (Utilities|String|ToString(Integer) _returnvalue_5))
  (bind _output (Utilities|Array|Get(acopy) _discoveredtilesortibgcost _returnvalue_5))
  (bind _returnvalue_7 (Utilities|String|ToString(Integer) _output))
  (bind _returnvalue_8 (Utilities|String|Append "Sort:" _returnvalue_6 " (" _returnvalue_7 ")"))
  (if (CallFunction|WanttoDisplayAnyText)
    ;[0 0 0] Мы хотим писать текст только в том случае, если плитка действительна в данных сетки и если это плитка, по которой можно пройти.
    (if _returnvalue_3
      (bind _output_get (LocalVariables|SetData _value))
      (if (CallFunction|IsTileTypeWalkable (.type _output_get))
        (Utilities|FlowControl|Sequence
          (:then_0
            (Utilities|FlowControl|Sequence
              (:then_0
                (if (Variables|Default|GetShowTileIndexes)
                  (Utilities|Array|Add (LocalVariables|GetText) _returnvalue_4)
                  (Utilities|Array|Add (LocalVariables|GetText_Lengths) (Utilities|String|Len _returnvalue_4))))
              (:then_1
                (if (Math|Boolean|ORBoolean (Variables|Default|GetShowTileIndexes) (Variables|Default|GetShowCostToEnterTile) (Variables|Default|GetShowMinCostToTarget) (Variables|Default|GetShowCostFromStart) (Variables|Default|GetShowSortOrder))
                  (if (.ReturnValue (Utilities|Map|Find (Variables|/Game/Blueprints/Core/Grid/BP_GridPathfinding.BP_GridPathfinding_C|GetPathfindingData (Variables|/Game/Blueprints/Core/Grid/BP_Grid.BP_Grid_C|GetGridPathfinding (Variables|Default|GetGrid))) Index))
                    (LocalVariables|SetPathfindingData (.Value (Utilities|Map|Find (Variables|/Game/Blueprints/Core/Grid/BP_GridPathfinding.BP_GridPathfinding_C|GetPathfindingData (Variables|/Game/Blueprints/Core/Grid/BP_Grid.BP_Grid_C|GetGridPathfinding (Variables|Default|GetGrid))) Index)))
                    (Utilities|FlowControl|Sequence
                      (:then_0
                        (if (Variables|Default|GetShowCostToEnterTile)
                          (Utilities|Array|Add (LocalVariables|GetText) (Utilities|String|Append "Enter:" (Utilities|String|ToString(Integer) (Utilities|Struct|BreakS_PathfindingData (LocalVariables|GetPathfindingData)))))
                          (Utilities|Array|Add (LocalVariables|GetText_Lengths) (Utilities|String|Len (Utilities|String|Append "Enter:" (Utilities|String|ToString(Integer) (Utilities|Struct|BreakS_PathfindingData (LocalVariables|GetPathfindingData))))))))
                      (:then_1
                        (if (Variables|Default|GetShowMinCostToTarget)
                          (if (!= (Utilities|Struct|BreakS_PathfindingData (LocalVariables|GetPathfindingData)) 999999)
                            (Utilities|Array|Add (LocalVariables|GetText) (Utilities|String|Append "Min:" (Utilities|String|ToString(Integer) (Utilities|Struct|BreakS_PathfindingData (LocalVariables|GetPathfindingData)))))
                            (Utilities|Array|Add (LocalVariables|GetText_Lengths) (Utilities|String|Len (Utilities|String|Append "Min:" (Utilities|String|ToString(Integer) (Utilities|Struct|BreakS_PathfindingData (LocalVariables|GetPathfindingData)))))))))
                      (:then_2
                        (if (Variables|Default|GetShowCostFromStart)
                          (if (!= (Utilities|Struct|BreakS_PathfindingData (LocalVariables|GetPathfindingData)) 999999)
                            (Utilities|Array|Add (LocalVariables|GetText) (Utilities|String|Append "Start:" (Utilities|String|ToString(Integer) (Utilities|Struct|BreakS_PathfindingData (LocalVariables|GetPathfindingData)))))
                            (Utilities|Array|Add (LocalVariables|GetText_Lengths) (Utilities|String|Len (Utilities|String|Append "Start:" (Utilities|String|ToString(Integer) (Utilities|Struct|BreakS_PathfindingData (LocalVariables|GetPathfindingData)))))))))
                      (:then_3
                        (if (Variables|Default|GetShowSortOrder)
                          (if (!= _returnvalue_5 -1)
                            (Utilities|Array|Add (LocalVariables|GetText) _returnvalue_8)
                            (Utilities|Array|Add (LocalVariables|GetText_Lengths) (Utilities|String|Len _returnvalue_8)))))))))))
          (:then_1
            (if (> (Utilities|Array|Length (LocalVariables|GetText)) 0)
              (bind _textrenderactor (TextActor|GetTextActor Index))
              (LocalVariables|SetTextActor _textrenderactor)
              (Rendering|Components|TextRender|SetText (Variables|/Script/Engine.TextRenderActor|GetTextRender (LocalVariables|GetTextActor)) (Utilities|Text|ToText(String) (Utilities|String|JoinStringArray (LocalVariables|GetText) " 
 ")))
              (Transformation|SetActorTransform (LocalVariables|GetTextActor) (Math|Transform|MakeTransform (+ (.location (.transform (LocalVariables|GetData))) "0.000000,0.000000,1.000000") "90.000000,180.000000,0.000000" (Math|Conversions|ToVector(Float) (/ (.y (Variables|/Game/Blueprints/Core/Grid/BP_Grid.BP_Grid_C|GetGridTileSize (Variables|Default|GetGrid))) (* (.MaxValue (Math|Integer|MaxOfIntArray (LocalVariables|GetText_Lengths))) 15.0)))))
              (else
                (TextActor|DestroyTextActor Index)))))
        (else
          ;[0 0 0] Если плитки не существует или тип плитки, например препядствие, то текст будет уничтожен.
          (TextActor|DestroyTextActor Index :!label _label)))
      (else
        (goto _label)))))

(fn SetShowTileIndexes
  (params (ShowTileIndexes :type Boolean) (ShowCostToEnterTile :type Boolean) (ShowMinCostToTarget :type Boolean) (ShowCostFromStart :type Boolean) (ShowSortOrder :type Boolean))
  ;[0 0 0] Если мы показываем индексы плиток, мы обновляем все плитки, чтобы убедиться, что мы воссоздаем их, если они были уничтожены. В противном случае уничтожьте все тексты
  (Variables|Default|SetShowTileIndexes ShowTileIndexes)
  (Variables|Default|SetShowCostToEnterTile ShowCostToEnterTile)
  (Variables|Default|SetShowMinCostToTarget ShowMinCostToTarget)
  (Variables|Default|SetShowCostFromStart ShowCostFromStart)
  (Variables|Default|SetShowSortOrder ShowSortOrder)
  (CallFunction|UpdateTextonAllTiles))

(fn UpdateTextonAllTiles
  (if (CallFunction|WanttoDisplayAnyText)
    (bind _keys (Utilities|Map|Keys (Variables|/Game/Blueprints/Core/Grid/BP_Grid.BP_Grid_C|GetGridTiles (Variables|Default|GetGrid))))
    (for _array_element _keys
      (CallFunction|UpdateTextonTile _array_element))
    (else
      (TextActor|ClearAllTextActor))))

(fn WanttoDisplayAnyText
  (return (Math|Boolean|ORBoolean (Variables|Default|GetShowTileIndexes) (Variables|Default|GetShowCostToEnterTile) (Variables|Default|GetShowMinCostToTarget) (Variables|Default|GetShowCostFromStart) (Variables|Default|GetShowSortOrder))))