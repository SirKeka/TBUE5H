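; BP_GridVisual renders the grid's tiles through two instanced-mesh child actors: a flat overlay and a tactical view.
; Tile updates re-add flat instances for walkable types, raised by a ground offset.
; Tactical tiles are colored by type and Z-scaled down to the tracked lowest grid height.
; Toggling tactical mode hides actors tagged "NotTactical" and lazily regenerates tactical tiles flagged dirty while it was off.
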(event EventBeginPlay
  (Actor|Tick|SetActorTickEnabled false))

(event Collision|EventActorBeginOverlap
  (params (OtherActor :type Actor%20Object%20Reference)))

(event EventTick
  (params (DeltaSeconds :type Float%20%28single-precision%29)))

(fn ConstructionScript)

(fn InitializeGridVisual
  (params (Grid :type BP%20Grid%20Object%20Reference))
  ;[0 0 0] Настройте ссылку
  (Variables|Default|SetGrid Grid)
  (bind _output_get (Variables|Default|SetGridMeshInst (.AsBP%20Grid%20Mesh%20Inst (Utilities|Casting|CastToBP_gridMeshInst (Variables|/Script/Engine.ChildActorComponent|GetChildActor (Variables|Default|GetChildActor_GridMeshInst))))))
  (bind _output_get_2 (Variables|Default|SetGridMeshInst_Tactical (.AsBP%20Grid%20Mesh%20Inst (Utilities|Casting|CastToBP_gridMeshInst (Variables|/Script/Engine.ChildActorComponent|GetChildActor (Variables|Default|GetChildActor_GridMeshInst_Tactical))))))
  ;[0 0 0] Настройте компоненты
  (Default|InitializeGridMeshInst _output_get (.FlatMesh (Utilities|Struct|BreakS_GridShapeData (Default|GetCurrentShape (Variables|Default|GetGrid)))) (.FlatMaterial (Utilities|Struct|BreakS_GridShapeData (Default|GetCurrentShape (Variables|Default|GetGrid)))) false "QueryOnly")
  (Default|InitializeGridMeshInst _output_get_2 (.Mesh (Utilities|Struct|BreakS_GridShapeData (Default|GetCurrentShape (Variables|Default|GetGrid)))) (.MeshMaterial (Utilities|Struct|BreakS_GridShapeData (Default|GetCurrentShape (Variables|Default|GetGrid)))) true "QueryOnly")
  (Transformation|SetActorLocation "0, 0, 0" false false) ; Центральная сетка в мире
  (CallFunction|SetOffsetfromGround (Variables|Default|GetOffsetFromGround)) ; Установить высоту сетки
  (CallFunction|SetGridLowestZ 999999.0)
  (CallFunction|SetIsTactical (Variables|Default|GetIsTactical)))

(fn SetOffsetfromGround
  (params (Offset :type Float%20%28double-precision%29))
  ;[0 0 0] Установите высоту сетки, не трогайте X и Y
  (bind _output_get (Variables|Default|SetOffsetFromGround Offset))
  (Transformation|SetRelativeLocation (Variables|Default|GetChildActor_GridMeshInst) (Math|Vector|MakeVector 0.0 0.0 _output_get) false false))

(fn DestroyGridVisual
  (bind _gridmeshinst_tactical (Variables|Default|GetGridMeshInst_Tactical))
  (bind _gridmeshinst (Variables|Default|GetGridMeshInst))
  ;[0 0 0] Очистка экземпляров компонента
  (Utilities|FlowControl|Sequence
    (:then_0
      (Utilities|IsValid _gridmeshinst
        (:Is%20Valid
          (Default|ClearInstance _gridmeshinst))))
    (:then_1
      (Utilities|IsValid _gridmeshinst_tactical
        (:Is%20Valid
          (Default|ClearInstance _gridmeshinst_tactical))))
    (:then_2
      (CallFunction|SetGridLowestZ 999999.0))))

(fn UpdateTileVisual
  (params (Data :type S%20Tile%20Data%20Structure))
  ;[0 0 0] Обновление визуального элемента плитки на основе его данных
  (Utilities|FlowControl|Sequence
    (:then_0
      (Default|RemoveInstance (Variables|Default|GetGridMeshInst) (.index Data))
      (if (CallFunction|IsTileTypeWalkable (.type Data))
        (Default|AddInstance (Variables|Default|GetGridMeshInst) (.index Data) (.type Data) (.transform Data) (.states Data))))
    (:then_1
      (CallFunction|UpdateTileVisualTactical Data))))

(fn UpdateTileVisualTactical
  (params (Data :type S%20Tile%20Data%20Structure))
  (bind _grid (Variables|Default|GetGrid))
  (bind _location (Math|Transform|BreakTransform (.transform Data)))
  (bind (_location_2 _rotation _scale) (Math|Transform|BreakTransform (.transform Data)))
  (bind _returnvalue (Default|GetCurrentShape _grid))
  (bind _meshsize (Utilities|Struct|BreakS_GridShapeData _returnvalue))
  (bind _z (Math|Vector|BreakVector _meshsize))
  (Utilities|FlowControl|Sequence
    (:then_0
      (if (< (.z _location) (Variables|Default|GetGridLowestZ))
        (CallFunction|SetGridLowestZ (.z _location))))
    (:then_1
      (if (Variables|Default|GetIsTactical)
        (Default|RemoveInstance (Variables|Default|GetGridMeshInst_Tactical) (.index Data))
        (if (Utilities|Enum|NotEqual(Enum) (.type Data) "NewEnumerator0")
          (Default|AddInstance (Variables|Default|GetGridMeshInst_Tactical) (.index Data) (.type Data) (Math|Transform|MakeTransform _location_2 _rotation (Math|Vector|MakeVector (.x _scale) (.y _scale) (/ (+ (- (.Z (Math|Vector|BreakVector (.Location (Math|Transform|BreakTransform (.transform Data))))) (Variables|Default|GetGridLowestZ)) _z) _z))) (.states Data)))
        (else
          (Variables|Default|SetNeedToReGenerateTactical%20OnNextEnable true))))))

(fn SetGridLowestZ
  (params (Z :type Float%20%28double-precision%29))
  (Variables|Default|SetGridLowestZ Z)
  (Variables|Default|SetNeedToReGenerateTactical%20OnNextEnable true))

(fn SetIsTactical
  (params (Tactical :type Boolean))
  (bind _output_get (Variables|Default|SetIsTactical Tactical))
  (Development|SetHiddeninGame (Variables|Default|GetChildActor_GridMeshInst_Tactical) (not _output_get) false)
  (bind _outactors (Actor|GetAllActorswithTag "NotTactical"))
  (for _array_element _outactors
    (Rendering|SetActorHiddenInGame _array_element (Variables|Default|GetIsTactical)))
  (if (and (Variables|Default|GetIsTactical) (Variables|Default|GetNeedToReGenerateTactical%20OnNextEnable))
    (Variables|Default|SetNeedToReGenerateTactical%20OnNextEnable false)
    (bind _values (Utilities|Map|Values (Variables|/Game/Blueprints/Core/Grid/BP_Grid.BP_Grid_C|GetGridTiles (Variables|Default|GetGrid))))
    (for _array_element_2 _values
      (CallFunction|UpdateTileVisualTactical _array_element_2))))