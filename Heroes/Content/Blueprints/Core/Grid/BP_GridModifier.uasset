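; BP_GridModifier is a placeable volume that marks grid areas with a tile type, such as normal, obstacle, higher movement cost or flying units only.
; The Construction Script sets its mesh and flat material from Shape data and colors it by Type.
; It applies collision responses after SetStaticMesh, which resets them, so ground-channel traces detect the volume.
; The actor is hidden in game and has no active event logic.
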(event EventBeginPlay)

(event Collision|EventActorBeginOverlap
  (params (OtherActor :type Actor%20Object%20Reference)))

(event EventTick
  (params (DeltaSeconds :type Float%20%28single-precision%29)))

(fn ConstructionScript
  (bind _staticmesh (Variables|Default|GetStaticMesh))
  (bind _shape (Variables|Default|GetShape))
  (bind _staticmesh_2 (Variables|Default|GetStaticMesh))
  (bind _data (CallFunction|GetShapeData _shape))
  ;[0 0 0] Установите визуальный эффект объема в зависимости от формы и типа
  (Components|StaticMesh|SetStaticMesh _staticmesh_2 (.mesh _data))
  (Rendering|Material|SetMaterial _staticmesh_2 0 (.flatmaterial _data))
  (Rendering|Material|SetVectorParameterValueonMaterials _staticmesh_2 "Color" (Math|Conversions|ToVector(LinearColor) (Utilities|Select :Index (Variables|Default|GetType) :NewEnumerator0 "" :NewEnumerator1 "(R=1.000000,G=1.000000,B=1.000000,A=1.000000)" :NewEnumerator2 "(R=0.700000,G=0.000000,B=0.009115,A=1.000000)" :NewEnumerator3 "(R=0.588542,G=0.571869,B=0.238236,A=1.000000)" :NewEnumerator4 "(R=1.000000,G=0.608315,B=0.113053,A=1.000000)" :NewEnumerator5 "(R=0.250597,G=0.281691,B=0.776042,A=1.000000)")))
  (Rendering|Material|SetScalarParameterValueonMaterials _staticmesh_2 "IsFilled" 1.0)
  ;[0 0 0] Объем должен перекрывать тот же канал трассировки, что и земля. Мы должны установить его после настройки сетки, потому что функция SetStaticMesh сбрасывает эту настройку.
  (Collision|SetCollisionResponsetoChannel _staticmesh "ECC_GameTraceChannel1" "ECR_Overlap")
  (Collision|SetCollisionResponsetoChannel _staticmesh "ECC_GameTraceChannel4" "ECR_Block")
  (Rendering|SetActorHiddenInGame true))