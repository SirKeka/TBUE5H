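; Grid visual actor that draws tiles through one InstancedStaticMesh, with mesh, material, collision and color mode set on initialization.
; AddInstance replaces any instance for that tile index, using the parallel InstanceIndexes array to map tiles to instances.
; GetColorFromStates picks color by tile type or by the highest-priority tile state.
; RGB and an IsFilled flag reach the material through four per-instance custom data floats.
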(event EventBeginPlay
  (Actor|Tick|SetActorTickEnabled false))

(event Collision|EventActorBeginOverlap
  (params (OtherActor :type Actor%20Object%20Reference)))

(event EventTick
  (params (DeltaSeconds :type Float%20%28single-precision%29)))

(fn ConstructionScript)

(fn AddInstance
  (params (Index :type Int%20Point%20Structure%20%28by%20ref%29) (TileType :type E_TileType%20Enum :default "NewEnumerator0") (Transform :type Transform%20%28by%20ref%29) (States :type Array%20of%20E_TileState%20Enums :default "NewEnumerator0"))
  (bind _instancedstaticmesh (Variables|Default|GetInstancedStaticMesh))
  ;[0 0 0] Сначала удалите экземпляр, потому что у нас может быть только одна плитка для каждого индекса. Затем обновите преобразование и добавьте его в массив для будущего доступа.
  (CallFunction|RemoveInstance Index)
  (Components|InstancedStaticMesh|AddInstance (Variables|Default|GetInstancedStaticMesh) Transform false)
  (bind _returnvalue (Utilities|Array|Add (Variables|Default|GetInstanceIndexes) Index))
  (bind _output_get (LocalVariables|SetI _returnvalue))
  ;[0 0 0] Используйте CustomDataValue (Пользовательское значение данныхПользовательское значение данных), чтобы установить цвета для конкретных плиток, которые нам нужны — ВАЖНО! - Обязательно установите для NumCustomDataFloat (Количество пользовательских данных с плавающей запятой) значение 4 в компоненте.
  ;
  ; 0 = Заполнено | 1=R | 2=G | 3=B
  (bind (_color _isfilled) (CallFunction|GetColorfromStates TileType States))
  (Components|InstancedStaticMesh|SetCustomDataValue _instancedstaticmesh _output_get 0 (.R (Math|Color|BreakColor _color)) false) ; 0 = Заполнено
  (Components|InstancedStaticMesh|SetCustomDataValue _instancedstaticmesh _output_get 1 (.G (Math|Color|BreakColor _color)) false) ; 1 = R
  (Components|InstancedStaticMesh|SetCustomDataValue _instancedstaticmesh _output_get 2 (.B (Math|Color|BreakColor _color)) false) ; 2 = G
  (Components|InstancedStaticMesh|SetCustomDataValue _instancedstaticmesh _output_get 3 _isfilled false) ; 3 =B
)

(fn RemoveInstance
  (params (ItemToFind :type Int%20Point%20Structure%20%28by%20ref%29))
  (bind _instanceindexes (Variables|Default|GetInstanceIndexes))
  (if (Utilities|Array|ContainsItem _instanceindexes ItemToFind)
    (Class|InstancedStaticMeshComponent|RemoveInstance (Variables|Default|GetInstancedStaticMesh) (Utilities|Array|FindItem _instanceindexes ItemToFind))
    (Utilities|Array|RemoveItem (Variables|Default|GetInstanceIndexes) ItemToFind)))

(fn ClearInstance
  (Components|InstancedStaticMesh|ClearInstances (Variables|Default|GetInstancedStaticMesh))
  (Utilities|Array|Clear (Variables|Default|GetInstanceIndexes)))

(fn InitializeGridMeshInst
  (params (Mesh :type Static%20Mesh%20Object%20Reference) (Material :type Material%20Interface%20Object%20Reference) (ColorBasedOnTileType :type Boolean) (Collision :type ECollisionEnabled%20Enum :default "NoCollision"))
  (bind _instancedstaticmesh (Variables|Default|GetInstancedStaticMesh))
  ;[0 0 0] Устанавливает данные по умолчанию, необходимые для отображения этой сетки
  (Components|StaticMesh|SetStaticMesh _instancedstaticmesh Mesh)
  (Rendering|Material|SetMaterial _instancedstaticmesh 0 Material)
  (Variables|Default|SetIsColorBasedOnTileType ColorBasedOnTileType)
  (Collision|SetCollisionEnabled _instancedstaticmesh Collision))

(fn GetColorfromStates
  (params (TileType :type E_TileType%20Enum :default "NewEnumerator0") (States :type Array%20of%20E_TileState%20Enums :default "NewEnumerator0"))
  ;[0 0 0] Основываясь на состояниях плитки, верните первый цвет, который мы нашли в нашем списке приоритетов.
  (if (Variables|Default|GetIsColorBasedOnTileType)
    (return (Utilities|Select :Index TileType :NewEnumerator0 "" :NewEnumerator1 "(R=0.250000,G=0.500000,B=0.255597,A=1.000000)" :NewEnumerator2 "(R=0.859375,G=0.062663,B=0.157272,A=1.000000)" :NewEnumerator3 "(R=0.188235,G=0.749020,B=0.200000,A=1.000000)" :NewEnumerator4 "(R=0.000000,G=1.000000,B=0.020979,A=1.000000)" :NewEnumerator5 "(R=0.117209,G=0.620854,B=0.880208,A=1.000000)") 1.0)
    (elif (== (Utilities|Array|Length States) 0)
      (return "" 0.0)
      (else
        (for _array_element (Utilities|Array|MakeArray "NewEnumerator9" "NewEnumerator8" "NewEnumerator2" "NewEnumerator1" "NewEnumerator3" "NewEnumerator4" "NewEnumerator5" "NewEnumerator6" "NewEnumerator7")
          (if (Utilities|Array|ContainsItem States _array_element)
            (return (Utilities|Select :Index _array_element :NewEnumerator0 "" :NewEnumerator1 "(R=0.500000,G=0.441414,B=0.000000,A=1.000000)" :NewEnumerator2 "(R=0.500000,G=0.258202,B=0.062098,A=1.000000)" :NewEnumerator3 "(R=0.189238,G=1.000000,B=0.363788,A=1.000000)" :NewEnumerator4 "(R=0.200000,G=0.807301,B=1.000000,A=1.000000)" :NewEnumerator5 "(R=1.000000,G=0.047059,B=0.137255,A=1.000000)" :NewEnumerator6 "(R=0.500000,G=0.000000,B=0.047325,A=1.000000)" :NewEnumerator7 "(R=0.000000,G=0.085409,B=0.677083,A=1.000000)" :NewEnumerator8 "(R=0.250000,G=0.132531,B=0.062500,A=1.000000)" :NewEnumerator9 "(R=0.250000,G=0.056239,B=0.058228,A=1.000000)") 1.0)))
        (return "" 0.0)))))