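; Grid pathfinding component that runs A* over square or hexagonal tiles to return a path or the reachable tiles within a cost limit.
; Neighbors are filtered by tile type, occupancy and height step (ignored for flyers), with weighted entry costs.
; A cost-sorted open list favors straight steps on ties.
; Searches run synchronously or time-sliced through a gated delay loop, firing callbacks for data updates and completion.
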(event Custom|FindPathWithDelay
  ;[0 0 0] Нам нужны ворота на тот случай, если нам нужно остановить поток. (например, если мы начнем новый путь до того, как он завершится по таймеру)
  (Utilities|FlowControl|Sequence
    (:then_0
      (goto _label_3 Open))
    (:then_1
      ;[0 0 0] Запомните время в начале, чтобы мы знали, потратили ли мы слишком много времени на текущую итерацию.
      (Variables|GeneratedData|SetLoopStartTime (Math|DateTime|Now) :!label _label)
      ;[0 0 0] Обычная логика поиска путей
      (if (> (Utilities|Array|Length (Variables|GeneratedData|GetDiscoveredTileIndexes)) 0) :!label _label_2
        (bind _foundtargettile (CallFunction|AnalyseNextDiscoveredTile))
        (if _foundtargettile
          (bind _path (Utilities|GeneratePath))
          (Default|CallOnPathfindingCompleted _path)
          (else
            (if (> (Variables|Default|GetDelayBetweenItteration) 0.0)
              (if (< (Class|KismetMathLibrary|GetTotalMilliseconds (- (Math|DateTime|Now) (Variables|GeneratedData|GetLoopStartTime))) (Variables|Default|GetMaxMsPerFrame))
                (goto _label_2)
                (else
                  _)))
            ;[0 0 0] Подождите немного перед следующей итерацией
            (Utilities|FlowControl|RetriggerableDelay (Variables|Default|GetDelayBetweenItteration))
            (Utilities|FlowControl|Gate true :!label _label_3
              (:Exit
                (goto _label)))))
        (else
          (Default|CallOnPathfindingCompleted (select (Variables|Default|GetReturnReachablesTile) (Variables|GeneratedData|GetAnalysedTileIndexes) (Utilities|Array|MakeArray))))))))

(event Custom|CloseDelayGate
  ;[0 0 0] Нам нужны ворота на тот случай, если нам нужно остановить поток. (например, если мы начнем новый путь до того, как он завершится по таймеру)
  (Utilities|FlowControl|Gate true) ; enters at Close
)

(event EventBeginPlay)

(event Collision|EventActorBeginOverlap
  (params (OtherActor :type Actor%20Object%20Reference)))

(event EventTick
  (params (DeltaSeconds :type Float%20%28single-precision%29)))

(fn ConstructionScript)

(fn GetValidTileHeighbors
  (params (Index :type Int%20Point%20Structure) (IncludeDiagonals :type Boolean) (ValidTypes :type Array%20of%20E_TileType%20Enums :default "NewEnumerator0"))
  ;[0 0 0] Чтобы сравнить высоту позже
  (LocalVariables|SetInputData (.Value (Utilities|Map|Find (Variables|/Game/Blueprints/Core/Grid/BP_Grid.BP_Grid_C|GetGridTiles (Variables|Default|GetGrid)) Index)))
  ;[0 0 0] Перебрать всех потенциальных соседей, чтобы проверить их
  (bind _neighbors (Neighbors|GetHeighborIndexes Index IncludeDiagonals))
  (for _array_element _neighbors
    (bind _output_get (LocalVariables|SetData (.Value (Utilities|Map|Find (Variables|/Game/Blueprints/Core/Grid/BP_Grid.BP_Grid_C|GetGridTiles (Variables|Default|GetGrid)) _array_element))))
    ;[0 0 0] Если это не проходимо, сосед недействителен
    (if (Utilities|Array|ContainsItem ValidTypes (.type _output_get))
      (if (not (Utilities|IsValid (Utilities|Struct|BreakS_TileData (LocalVariables|GetData))))
        (if (Variables|Default|GetIncludeFlyingOnly)
          ;[0 0 0] Действительный сосед!
          (Utilities|Array|Add (LocalVariables|GetRet) (Utilities|Struct|MakeS_PathfindingData (.index (LocalVariables|GetData)) (Utilities|Select :Index (.type (LocalVariables|GetData)) :NewEnumerator0 0 :NewEnumerator1 1 :NewEnumerator2 0 :NewEnumerator3 2 :NewEnumerator4 3 :NewEnumerator5 1) 999999 999999 Index) :!label _label)
          (else
            ;[0 0 0] Сравните разницу высот между текущей плиткой и соседней. Если он слишком большой, это недопустимый сосед.
            (if (<= (Math|Float|Absolute(Float) (- (.z (.location (.transform (LocalVariables|GetData)))) (.z (.location (.transform (LocalVariables|GetInputData)))))) 52.0)
              (goto _label)))))))
  (return (LocalVariables|GetRet)))

(fn GetNeighborIndexesforSquare
  (params (Index :type Int%20Point%20Structure) (IncludeDiagonals :type Boolean))
  (bind _intpoint (Utilities|Struct|MakeIntPoint 1 0))
  (bind _intpoint_2 (Utilities|Struct|MakeIntPoint 0 1))
  (bind _intpoint_3 (Utilities|Struct|MakeIntPoint -1 0))
  (bind _intpoint_4 (Utilities|Struct|MakeIntPoint 0 -1))
  (bind _returnvalue (+ Index _intpoint))
  (bind _returnvalue_2 (+ Index _intpoint_2))
  (bind _returnvalue_3 (+ Index _intpoint_3))
  (bind _returnvalue_4 (+ Index _intpoint_4))
  (bind _array (Utilities|Array|MakeArray _returnvalue _returnvalue_2 _returnvalue_3 _returnvalue_4))
  (if IncludeDiagonals
    (bind _output_get (LocalVariables|SetRet _array))
    (Utilities|Array|AppendArray _output_get (Utilities|Array|MakeArray (+ Index (Utilities|Struct|MakeIntPoint 1 1)) (+ Index (Utilities|Struct|MakeIntPoint -1 1)) (+ Index (Utilities|Struct|MakeIntPoint -1 -1)) (+ Index (Utilities|Struct|MakeIntPoint 1 -1))))
    (return (LocalVariables|GetRet))
    (else
      (return _array))))

(fn GetNeighborIndexesforHexagon
  (params (Index :type Int%20Point%20Structure))
  (return (Utilities|Array|MakeArray (+ Index (Utilities|Struct|MakeIntPoint 1 1)) (+ Index (Utilities|Struct|MakeIntPoint 0 2)) (+ Index (Utilities|Struct|MakeIntPoint -1 1)) (+ Index (Utilities|Struct|MakeIntPoint -1 -1)) (+ Index (Utilities|Struct|MakeIntPoint 0 -2)) (+ Index (Utilities|Struct|MakeIntPoint 1 -1)))))

(fn GetHeighborIndexes
  (params (Index :type Int%20Point%20Structure) (IncludeDiagonals :type Boolean))
  (switch Utilities|FlowControl|Switch|SwitchonE_GridShape (Variables|/Game/Blueprints/Core/Grid/BP_Grid.BP_Grid_C|GetGridShape (Variables|Default|GetGrid))
    (:NewEnumerator1
      (return (Neighbors|GetNeighborIndexesforSquare Index IncludeDiagonals)))
    (:NewEnumerator2
      (return (Neighbors|GetNeighborIndexesforHexagon Index)))))

(fn FindPath
  (params (Start :type Int%20Point%20Structure) (Target :type Int%20Point%20Structure) (Diagonals :type Boolean) (TileTypes :type Array%20of%20E_TileType%20Enums :default "NewEnumerator0") (Delay :type Float%20%28double-precision%29) (MaxMs :type Float%20%28double-precision%29) (ReturnReachables :type Boolean) (PathLenght :type Integer) (IncludeFlyingOnly :type Boolean))
  (bind _array (Utilities|Array|MakeArray))
  ;[0 0 0] Инициализируйте данные и убедитесь, что они действительны
  (Variables|Default|SetStartIndex Start)
  (Variables|Default|SetTargetIndex Target)
  (Variables|Default|SetIncludeDiagonals Diagonals)
  (Variables|Default|SetValid%20Types TileTypes)
  (Variables|Default|SetDelayBetweenItteration Delay)
  (Variables|Default|SetMaxMsPerFrame MaxMs)
  (Variables|Default|SetReturnReachablesTile ReturnReachables)
  (Variables|Default|SetMaxPathLenght PathLenght)
  (Variables|Default|SetIncludeFlyingOnly IncludeFlyingOnly)
  (CallFunction|CloseDelayGate)
  (Utilities|ClearGeneratedData)
  (bind _isvalid (Utilities|IsInputDataValid))
  (if _isvalid
    ;[0 0 0] Откройте для себя первую плитку (начальный индекс)
    (Utilities|DiscoverTile (Utilities|Struct|MakeS_PathfindingData (Variables|Default|GetStartIndex) 1 0 (Utilities|GetMinimumCostBetweenTiles (Variables|Default|GetStartIndex) (Variables|Default|GetTargetIndex) (Variables|Default|GetIncludeDiagonals)) "(X=-999,Y=-999)"))
    (if (<= (Variables|Default|GetDelayBetweenItteration) 0.0)
      ;[0 0 0] Пока у нас есть тайлы в списке Discovered, мы их анализируем. (Пока не найдем целевую плитку)
      (while (> (Utilities|Array|Length (Variables|GeneratedData|GetDiscoveredTileIndexes)) 0)
        (bind _foundtargettile (CallFunction|AnalyseNextDiscoveredTile))
        (if _foundtargettile
          ;[0 0 0] Целевая плитка найдена. Возврат пути
          (bind _path (Utilities|GeneratePath))
          (Default|CallOnPathfindingCompleted _path)
          (return _path) ; Путь найден
        ))
      ;[0 0 0] Целевая плитка не найдена. Невозможен путь от StartIndex к TargetIndex
      (Default|CallOnPathfindingCompleted (select (Variables|Default|GetReturnReachablesTile) (Variables|GeneratedData|GetAnalysedTileIndexes) (Utilities|Array|MakeArray)))
      (return (select (Variables|Default|GetReturnReachablesTile) (Variables|GeneratedData|GetAnalysedTileIndexes) (Utilities|Array|MakeArray))) ; Путь не найден
      (else
        (CallFunction|FindPathwithDelay)
        (return (Utilities|Array|MakeArray)) ; Путь не найден
      ))
    (else
      (Default|CallOnPathfindingCompleted _array)
      (return _array))))

(fn IsInputDataValid
  (bind _grid (Variables|Default|GetGrid))
  (bind _targetindex (Variables|Default|GetTargetIndex))
  (bind _gridtiles (Variables|/Game/Blueprints/Core/Grid/BP_Grid.BP_Grid_C|GetGridTiles _grid))
  (bind _value (Utilities|Map|Find _gridtiles _targetindex))
  (bind (_type _unitontile) (Utilities|Struct|BreakS_TileData _value))
  ;[0 0 0] Плитка действительна, если: Они не одинаковы и по обеим можно пройти.
  (if (!= (Variables|Default|GetStartIndex) (Variables|Default|GetTargetIndex))
    (if (not (Variables|Default|GetReturnReachablesTile))
      (if (Default|IsTileWalkable (Variables|Default|GetGrid) (Variables|Default|GetStartIndex))
        (if (<= (Utilities|GetMinimumCostBetweenTiles (Variables|Default|GetStartIndex) (Variables|Default|GetTargetIndex) (Variables|Default|GetIncludeDiagonals)) (Variables|Default|GetMaxPathLenght))
          (if (Utilities|Array|ContainsItem (Variables|Default|GetValid%20Types) _type)
            (if (not (Utilities|IsValid _unitontile))
              (return true)
              (else
                (return false)))
            (else
              (return false)))
          (else
            (return false)))
        (else
          (return false)))
      (else
        (return true)))
    (else
      (return false))))

(fn DiscoverTile
  (params (TilePathData :type S%20Pathfinding%20Data%20Structure))
  (bind _index (Utilities|Struct|BreakS_PathfindingData TilePathData))
  ;[0 0 0] Добавить плитку в данные и в списки обнаруженных
  (Utilities|Map|Add (Variables|GeneratedData|GetPathfindingData) _index TilePathData)
  (Utilities|InsertTileinDiscoveredArray TilePathData)
  (Default|CallOnPathfindingDataUpdated _index))

(fn GetMinimumCostBetweenTiles
  (params (Index1 :type Int%20Point%20Structure) (Index2 :type Int%20Point%20Structure) (Diagonal :type Boolean))
  (bind _returnvalue (- Index1 Index2))
  (bind _returnvalue_2 (- Index1 Index2))
  (bind _returnvalue_3 (- Index1 Index2))
  (bind _returnvalue_4 (Math|Integer|Absolute(Integer) (.x _returnvalue)))
  (switch Utilities|FlowControl|Switch|SwitchonE_GridShape (Variables|/Game/Blueprints/Core/Grid/BP_Grid.BP_Grid_C|GetGridShape (Variables|Default|GetGrid))
    (:NewEnumerator1
      (if Diagonal
        (return (Math|Integer|Max(Integer) (Math|Integer|Absolute(Integer) (.x _returnvalue_2)) (Math|Integer|Absolute(Integer) (.y _returnvalue_2))))
        (else
          (return (+ (Math|Integer|Absolute(Integer) (.x _returnvalue_3)) (Math|Integer|Absolute(Integer) (.y _returnvalue_3)))))))
    (:NewEnumerator2
      (return (+ _returnvalue_4 (Math|Integer|Max(Integer) (/ (- (Math|Integer|Absolute(Integer) (.y _returnvalue)) _returnvalue_4) 2)))))))

(fn AnalyseNextDiscoveredTile
  ;[0 0 0] Всегда обрабатывать самый дешевый
  (bind _tilepathdata (Utilities|PullCheapestTileOutOfDiscoveredList))
  (bind _output_get (Variables|GeneratedData|SetCurrentDiscoveredTile _tilepathdata))
  (Default|CallOnPathfindingDataUpdated (Utilities|Struct|BreakS_PathfindingData _output_get))
  (bind _neighbors (Neighbors|GetValidTileHeighbors (Utilities|Struct|BreakS_PathfindingData _output_get) (Variables|Default|GetIncludeDiagonals) (Variables|Default|GetValid%20Types)))
  (bind _output_get_2 (Variables|GeneratedData|SetCurrentNeighbors _neighbors))
  (while (> (Utilities|Array|Length _output_get_2) 0)
    (bind _istargettile (CallFunction|DiscoverNextNeighbor))
    (if _istargettile
      (return true) ; Этот сосед является целью
    ))
  (return false) ; Ни один из соседей не был целевой плиткой
)

(fn GeneratePath
  ;[0 0 0] Получите путь от TargetIndex обратно к StartIndex. Затем переверните его, чтобы он был правильным
  (bind _output_get (LocalVariables|SetCurrent (Variables|Default|GetTargetIndex)))
  (while (!= _output_get (Variables|Default|GetStartIndex))
    (Utilities|Array|Add (LocalVariables|GetInvertedPath) (LocalVariables|GetCurrent))
    (LocalVariables|SetCurrent (Utilities|Struct|BreakS_PathfindingData (.Value (Utilities|Map|Find (Variables|GeneratedData|GetPathfindingData) (LocalVariables|GetCurrent))))))
  (bind _arrayelement (Utilities|Array|ReverseforEachLoop (LocalVariables|GetInvertedPath))
    (:LoopBody
      (Utilities|Array|Add (LocalVariables|GetRet) _arrayelement))
    (:Completed
      (return (LocalVariables|GetRet)))))

(fn PullCheapestTileOutOfDiscoveredList
  (LocalVariables|SetTileIndex (Utilities|Array|Get(acopy) (Variables|GeneratedData|GetDiscoveredTileIndexes)))
  (Utilities|Array|RemoveIndex (Variables|GeneratedData|GetDiscoveredTileSortibgCost))
  (Utilities|Array|RemoveIndex (Variables|GeneratedData|GetDiscoveredTileIndexes))
  (Utilities|Array|Add (Variables|GeneratedData|GetAnalysedTileIndexes) (LocalVariables|GetTileIndex))
  (return (.Value (Utilities|Map|Find (Variables|GeneratedData|GetPathfindingData) (LocalVariables|GetTileIndex)))))

(fn DiscoverNextNeighbor
  ;[0 0 0] Получите первого соседа, чтобы обнаружить.
  (Variables|GeneratedData|SetCurrentNeighbor (Utilities|Array|Get(acopy) (Variables|GeneratedData|GetCurrentNeighbors)))
  (Utilities|Array|RemoveIndex (Variables|GeneratedData|GetCurrentNeighbors))
  ;[0 0 0] Продолжайте поток, только если мы еще не проанализировали его
  (if (not (Utilities|Array|ContainsItem (Variables|GeneratedData|GetAnalysedTileIndexes) (Utilities|Struct|BreakS_PathfindingData (Variables|GeneratedData|GetCurrentNeighbor)))) ; Еще не проанализировано
    (bind _output_get (LocalVariables|SetCostFromStart (+ (Utilities|Struct|BreakS_PathfindingData (Variables|GeneratedData|GetCurrentDiscoveredTile)) (Utilities|Struct|BreakS_PathfindingData (Variables|GeneratedData|GetCurrentNeighbor)))))
    (if (<= _output_get (Variables|Default|GetMaxPathLenght))
      ;[0 0 0] Еще не в списке обнаруженных? Значит, это новый сосед. Мы можем просто обнаружить это
      (bind _output_get_2 (LocalVariables|SetIndexInDiscovered (Utilities|Array|FindItem (Variables|GeneratedData|GetDiscoveredTileIndexes) (Utilities|Struct|BreakS_PathfindingData (Variables|GeneratedData|GetCurrentNeighbor)))))
      (if (== _output_get_2 -1) ; Новый сосед?
        _
        (else
          (bind _output_get_3 (Variables|GeneratedData|SetCurrentNeighbor (.Value (Utilities|Map|Find (Variables|GeneratedData|GetPathfindingData) (Utilities|Struct|BreakS_PathfindingData (Variables|GeneratedData|GetCurrentNeighbor))))))
          (if (< (LocalVariables|GetCostFromStart) (Utilities|Struct|BreakS_PathfindingData _output_get_3)) ; Нашли лучший путь к соседу?
            (Utilities|Array|RemoveIndex (Variables|GeneratedData|GetDiscoveredTileIndexes) (LocalVariables|GetIndexInDiscovered))
            (Utilities|Array|RemoveIndex (Variables|GeneratedData|GetDiscoveredTileSortibgCost) (LocalVariables|GetIndexInDiscovered))
            (else
              (return false)))))
      (Utilities|DiscoverTile (Utilities|Struct|MakeS_PathfindingData (.Index (Utilities|Struct|BreakS_PathfindingData (Variables|GeneratedData|GetCurrentNeighbor))) (.CostToEnterTile (Utilities|Struct|BreakS_PathfindingData (Variables|GeneratedData|GetCurrentNeighbor))) (LocalVariables|GetCostFromStart) (Utilities|GetMinimumCostBetweenTiles (Utilities|Struct|BreakS_PathfindingData (Variables|GeneratedData|GetCurrentNeighbor)) (Variables|Default|GetTargetIndex) (Variables|Default|GetIncludeDiagonals)) (Utilities|Struct|BreakS_PathfindingData (Variables|GeneratedData|GetCurrentDiscoveredTile))))
      (if (Class|KismetMathLibrary|EqualIntPointIntPoint (Utilities|Struct|BreakS_PathfindingData (Variables|GeneratedData|GetCurrentNeighbor)) (Variables|Default|GetTargetIndex))
        (return true)
        (else
          (return false)))
      (else
        (return false)))
    (else
      (return false))))

(fn InsertTileinDiscoveredArray
  (params (TileData :type S%20Pathfinding%20Data%20Structure))
  (bind _discoveredtilesortibgcost (Variables|GeneratedData|GetDiscoveredTileSortibgCost))
  ;[0 0 0] Вставьте плитку в правильное положение в массиве. Сортировка от самого дешевого до самого дорогого. Таким образом, в следующий раз, когда мы попытаемся найти самую дешевую плитку, мы можем просто взять индекс 0.
  (bind _output_get (LocalVariables|SetSortingCost (Utilities|GetTileSortingCost TileData)))
  (if (== (Utilities|Array|Length (Variables|GeneratedData|GetDiscoveredTileSortibgCost)) 0)
    (Utilities|Array|Add (Variables|GeneratedData|GetDiscoveredTileSortibgCost) _output_get :!label _label)
    (Utilities|Array|Add (Variables|GeneratedData|GetDiscoveredTileIndexes) (Utilities|Struct|BreakS_PathfindingData TileData))
    (elif (>= (LocalVariables|GetSortingCost) (Utilities|Array|Get(acopy) _discoveredtilesortibgcost (Utilities|Array|LastIndex _discoveredtilesortibgcost)))
      (goto _label)
      (else
        (bind (_array_element _array_index) (Utilities|Array|ForEachLoopwithBreak (Variables|GeneratedData|GetDiscoveredTileSortibgCost) :!label _label_2)
          (:LoopBody
            (if (>= _array_element (LocalVariables|GetSortingCost))
              (Utilities|Array|Insert (Variables|GeneratedData|GetDiscoveredTileSortibgCost) (LocalVariables|GetSortingCost) _array_index)
              (Utilities|Array|Insert (Variables|GeneratedData|GetDiscoveredTileIndexes) (Utilities|Struct|BreakS_PathfindingData TileData) _array_index)
              (goto _label_2 Break))))))))

(fn ClearGeneratedData
  ;[0 0 0] Просто очистите все, чтобы каждый поиск пути был чистым
  (Utilities|Map|Clear (Variables|GeneratedData|GetPathfindingData))
  (Utilities|Array|Clear (Variables|GeneratedData|GetDiscoveredTileSortibgCost))
  (Utilities|Array|Clear (Variables|GeneratedData|GetDiscoveredTileIndexes))
  (Utilities|Array|Clear (Variables|GeneratedData|GetAnalysedTileIndexes))
  (Default|CallOnPathfindingDataCleared))

(fn IsDiagonal
  (params (Index1 :type Int%20Point%20Structure) (Index2 :type Int%20Point%20Structure))
  (bind _neighbors (Neighbors|GetHeighborIndexes Index1 false))
  (return (not (Utilities|Array|ContainsItem _neighbors Index2))))

(fn GetTileSortingCost
  (params (TileData :type S%20Pathfinding%20Data%20Structure%20%28by%20ref%29))
  (bind (_costfromstart _minimumcosttotarget) (Utilities|Struct|BreakS_PathfindingData TileData))
  (bind (_index _previousindex) (Utilities|Struct|BreakS_PathfindingData TileData))
  ;[0 0 0] Добавление диагонали только к поиску пути предпочтительнее использовать прямую линию, если это та же стоимость.
  (return (+ (* (+ _costfromstart _minimumcosttotarget) 2) (Utilities|IsDiagonal _index _previousindex))))