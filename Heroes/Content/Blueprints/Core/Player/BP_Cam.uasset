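; BP_Cam is a player-controlled camera that pans, zooms and rotates in yaw through a spring arm.
; Axis inputs move a desired location along the actor's forward and right vectors and adjust a clamped desired arm length, while button presses step the desired yaw left or right.
; Tick smooths the motion by interpolating actor location, rotation and arm length toward those targets, which BeginPlay seeds from the starting state.
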(event EventTick
  (params (DeltaSeconds :type Float%20%28single-precision%29))
  (bind _springarm (Variables|Default|GetSpringArm))
  ;[0.1 0.1 0.1] В каждом кадре интерполируйте данные о движениях камеры (чтобы сделать их более плавными) и применяйте их к фактической камере.
  (Variables|/Script/Engine.SpringArmComponent|SetTargetArmLength _springarm (Math|Interpolation|FInterpTo (Variables|/Script/Engine.SpringArmComponent|GetTargetArmLength _springarm) (Variables|Zoom|GetZoomDesired) (Utilities|Time|GetWorldDeltaSeconds) (Variables|Default|GetZoomInterp)))
  (Transformation|SetActorLocation (Math|Interpolation|VInterpTo (Transformation|GetActorLocation) (Variables|Location|GetLocationDesired) (Utilities|Time|GetWorldDeltaSeconds) (Variables|Default|GetLocationInterp)) false false)
  (Transformation|SetActorRotation (Math|Interpolation|RInterpTo (Transformation|GetActorRotation) (Variables|Rotation|GetRotationDesired) (Utilities|Time|GetWorldDeltaSeconds) (Variables|Default|GetRotationInterp))))

(event EventBeginPlay
  (Variables|Location|SetLocationDesired (Transformation|GetActorLocation))
  (Variables|Zoom|SetZoomDesired (Variables|/Script/Engine.SpringArmComponent|GetTargetArmLength (Variables|Default|GetSpringArm)))
  (Variables|Rotation|SetRotationDesired (Transformation|GetActorRotation)))

(event Input|ActionEvents|InputActionNewActionRotationLeft
  (params (Key :type Key%20Structure :default "None"))
  ;[0.1 0.1 0.1] Каждый раз, когда игрок нажимает на ввод, мы добавляем количество ввода к Rotation_Desired (желаемое вращение)
  (:Pressed
    (Variables|Rotation|SetRotationDesired (Math|Rotator|CombineRotators (Variables|Rotation|GetRotationDesired) (Math|Rotator|MakeRotator 0.0 0.0 (Variables|Default|GetRotationSpeed))))))

(event Input|ActionEvents|InputActionNewActionRotationRight
  (params (Key :type Key%20Structure :default "None"))
  ;[0.1 0.1 0.1] Каждый раз, когда игрок нажимает на ввод, мы добавляем количество ввода к Rotation_Desired (желаемое вращение)
  (:Pressed
    (Variables|Rotation|SetRotationDesired (Math|Rotator|CombineRotators (Variables|Rotation|GetRotationDesired) (Math|Rotator|MakeRotator 0.0 0.0 (- 0.0 (Variables|Default|GetRotationSpeed)))))))

(event Input|AxisEvents|InputAxisNewAxisZoom
  (params (AxisValue :type Float%20%28single-precision%29))
  ;[0.1 0.1 0.1] В каждом кадре мы добавляем количество входных данных к Zoom_Desire (Zoom Desired).
  ; Не забудьте зафиксировать результат, чтобы игрок не мог приближаться к Луне.
  (Variables|Zoom|SetZoomDesired (Math|Float|Clamp(Float) (+ (Variables|Zoom|GetZoomDesired) (* AxisValue (Variables|Default|GetZoomSpeed))) (Variables|Default|GetZoomMin) (Variables|Default|GetZoomMax))))

(event Input|AxisEvents|InputAxisNewAxisForward
  (params (AxisValue :type Float%20%28single-precision%29))
  ;[0.1 0.1 0.1] В каждом кадре мы добавляем количество входных данных к Location_Desire (желаемое местоположение).
  (Variables|Location|SetLocationDesired (+ (Variables|Location|GetLocationDesired) (* (* AxisValue (Variables|Default|GetLocationSpeed)) (Transformation|GetActorForwardVector)))))

(event Input|AxisEvents|InputAxisNewAxisRight
  (params (AxisValue :type Float%20%28single-precision%29))
  ;[0.1 0.1 0.1] В каждом кадре мы добавляем количество входных данных к Location_Desire (желаемое местоположение).
  (Variables|Location|SetLocationDesired (+ (Variables|Location|GetLocationDesired) (* (* AxisValue (Variables|Default|GetLocationSpeed)) (Transformation|GetActorRightVector)))))

(fn ConstructionScript)