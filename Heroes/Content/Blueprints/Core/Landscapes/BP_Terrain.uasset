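; BP_Terrain is a terrain actor that builds a flat, procedural grid mesh in its construction script.
; GenerateTerrain clears old arrays, lays out vertices centered on the actor's XY location, spaced by CellSize divided by vertex count, and draws debug points.
; It adds two triangles per quad, using the larger vertex count as row multiplier, then creates the TerrainMesh section.
; Perlin noise is present but unused.
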(event EventBeginPlay)

(event Collision|EventActorBeginOverlap
  (params (OtherActor :type Actor%20Object%20Reference)))

(event EventTick
  (params (DeltaSeconds :type Float%20%28single-precision%29)))

(fn ConstructionScript
  (CallFunction|GenerateTerrain (Variables|Default|GetX_VertexCount) (Variables|Default|GetY_VertexCount) (Variables|Default|GetCellSize)))

(fn GenerateTerrain
  (params (X_VeretexCount :type Integer) (Y_VertexCount :type Integer) (CellSize :type Float%20%28double-precision%29))
  (bind _triangles (Variables|Default|GetTriangles))
  (Variables|Default|SetX_VertexCount X_VeretexCount)
  (Variables|Default|SetY_VertexCount Y_VertexCount)
  (Variables|Default|SetCellSize CellSize)
  (CallFunction|DestroyTerrain)
  (LocalVariables|SetVertexCoord (- (Transformation|GetActorLocation) (Math|Vector|MakeVector (* (/ (Variables|Default|GetCellSize) (Variables|Default|GetX_VertexCount)) (/ (- (Variables|Default|GetX_VertexCount) 1) 2.0)) (* (/ (- (Variables|Default|GetY_VertexCount) 1) 2.0) (/ (Variables|Default|GetCellSize) (Variables|Default|GetY_VertexCount))) 0.0)))
  (for _index (range 0 (- (Variables|Default|GetY_VertexCount) 1))
    (for _index_2 (range 0 (- (Variables|Default|GetX_VertexCount) 1))
      (Utilities|Array|Add (Variables|Default|GetVerices) (- (+ (LocalVariables|GetVertexCoord) (Math|Vector|MakeVector (* (/ (Variables|Default|GetCellSize) (Variables|Default|GetX_VertexCount)) _index_2) (* (/ (Variables|Default|GetCellSize) (Variables|Default|GetY_VertexCount)) _index) 0.0)) (Math|Vector|MakeVector 0.0 0.0 (.Z (Math|Vector|BreakVector (Transformation|GetActorLocation))))))
      (Rendering|Debug|DrawDebugPoint (+ (LocalVariables|GetVertexCoord) (Math|Vector|MakeVector (* (/ (Variables|Default|GetCellSize) (Variables|Default|GetX_VertexCount)) _index_2) (* (/ (Variables|Default|GetCellSize) (Variables|Default|GetY_VertexCount)) _index) 0.0)) 1e+01 "(R=1.000000,G=0.000000,B=0.000000,A=1.000000)" 1e+01)
      (if (and (< _index_2 (- (Variables|Default|GetX_VertexCount) 1)) (< _index (- (Variables|Default|GetY_VertexCount) 1)))
        ;[0 0 0] Левый нижний треугольник квадрата
        (Utilities|Array|Add _triangles (+ _index_2 (* _index (Math|Integer|SelectInt (Variables|Default|GetX_VertexCount) (Variables|Default|GetY_VertexCount) (> (Variables|Default|GetX_VertexCount) (Variables|Default|GetY_VertexCount))))))
        (Utilities|Array|Add _triangles (+ (+ _index_2 (* _index (Math|Integer|SelectInt (Variables|Default|GetX_VertexCount) (Variables|Default|GetY_VertexCount) (> (Variables|Default|GetX_VertexCount) (Variables|Default|GetY_VertexCount))))) (Variables|Default|GetX_VertexCount)))
        (Utilities|Array|Add _triangles (+ 1 (+ _index_2 (* _index (Math|Integer|SelectInt (Variables|Default|GetX_VertexCount) (Variables|Default|GetY_VertexCount) (> (Variables|Default|GetX_VertexCount) (Variables|Default|GetY_VertexCount)))))))
        ;[0 0 0] Правый верхний треугольник квадрата
        (Utilities|Array|Add _triangles (+ (+ _index_2 (* _index (Math|Integer|SelectInt (Variables|Default|GetX_VertexCount) (Variables|Default|GetY_VertexCount) (> (Variables|Default|GetX_VertexCount) (Variables|Default|GetY_VertexCount))))) (Variables|Default|GetX_VertexCount)))
        (Utilities|Array|Add _triangles (+ (+ _index_2 (* _index (Math|Integer|SelectInt (Variables|Default|GetX_VertexCount) (Variables|Default|GetY_VertexCount) (> (Variables|Default|GetX_VertexCount) (Variables|Default|GetY_VertexCount))))) (+ (Variables|Default|GetX_VertexCount) 1)))
        (Utilities|Array|Add _triangles (+ (+ _index_2 (* _index (Math|Integer|SelectInt (Variables|Default|GetX_VertexCount) (Variables|Default|GetY_VertexCount) (> (Variables|Default|GetX_VertexCount) (Variables|Default|GetY_VertexCount))))) 1)))))
  (Class|ProceduralMeshComponent|CreateMeshSectionLinearColor (Variables|Default|GetTerrainMesh) 0 (Variables|Default|GetVerices) (Variables|Default|GetTriangles) 0 0 0 0 0 0 0 false false))

(fn DestroyTerrain
  (Utilities|Array|Clear (Variables|Default|GetVerices))
  (Utilities|Array|Clear (Variables|Default|GetTriangles)))