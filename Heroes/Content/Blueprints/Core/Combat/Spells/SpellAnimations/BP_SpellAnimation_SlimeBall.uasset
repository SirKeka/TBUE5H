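; Spell animation actor that throws a green slime ball from the origin tile to the target tile.
; A timeline interpolates its position with a vertical offset while animating scale and the opacity of three spheres.
; Late in playback it reports a hit once for each attacked tile, then completes the spell animation when the timeline finishes.
; The construction script tints each sphere a different shade of green.
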(event EventEventPlaySpellAnimation
  (Transformation|SetActorLocation (.location (CallFunction|GetTileTransform (Variables|Default|GetOriginIndex))) false false)
  (bind (_direction _alpha _locationz _opacity _scale) (Timeline|Timeline_SlimeBall PlayFromStart)
    (:Update
      (Transformation|SetActorLocation (+ (Math|Vector|Lerp(Vector) (.location (CallFunction|GetTileTransform (Variables|Default|GetOriginIndex))) (.location (CallFunction|GetTileTransform (Variables|Default|GetTargetIndex))) _alpha) (Math|Vector|MakeVector 0.0 0.0 _locationz)) false false)
      (Rendering|Material|SetScalarParameterValueonMaterials (Variables|Default|GetSphere) "Opacity" _opacity)
      (Transformation|SetRelativeScale3D (Variables|Default|GetAnim_Scale) _scale)
      (if (>= (Components|Timeline|GetPlaybackPosition (Variables|Default|GetTimeline_SlimeBall)) 0.6)
        (Utilities|FlowControl|DoOnce false
          (:Completed
            (for _array_element (Variables|Default|GetAttackedIndexes)
              (Default|CallOnSpellAnimationHitTile self _array_element))))))
    (:Finished
      (CallFunction|EventCompleteSpellAnimation))))

(fn ConstructionScript
  (|CallParentFunction)
  (Rendering|Material|SetVectorParameterValueonMaterials (Variables|Default|GetSphere) "Color" (Math|Conversions|ToVector(LinearColor) "(R=0.011061,G=0.250000,B=0.059537,A=1.000000)"))
  (Rendering|Material|SetVectorParameterValueonMaterials (Variables|Default|GetSphere1) "Color" (Math|Conversions|ToVector(LinearColor) "(R=0.033183,G=0.750000,B=0.178611,A=1.000000)"))
  (Rendering|Material|SetVectorParameterValueonMaterials (Variables|Default|GetSphere2) "Color" (Math|Conversions|ToVector(LinearColor) "(R=0.022122,G=0.500000,B=0.119074,A=1.000000)")))