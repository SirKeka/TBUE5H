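; Spell animation actor for the Fireball spell, played between an origin tile and a target tile on the grid.
; When played, it snaps to the origin tile and faces the target, using the 2D tile indices for the look-at yaw.
; It then immediately, and only once, broadcasts the hit on the target tile and completes, with no travel or delay.
; The Fireball component's activate and deactivate calls are unconnected.
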(event EventBeginPlay
  (|CallParentFunction) ; This node is disabled and will not be called.\nDrag off pins to build functionality.
)

(event Collision|EventActorBeginOverlap
  (params (OtherActor :type Actor%20Object%20Reference)))

(event EventTick
  (params (DeltaSeconds :type Float%20%28single-precision%29)))

(event EventEventPlaySpellAnimation
  (Transformation|SetActorLocationAndRotation (.location (CallFunction|GetTileTransform (Variables|Default|GetOriginIndex))) (Math|Rotator|FindLookatRotation (Math|Conversions|ToVector(Vector2D) (Math|Conversions|ToVector2D(IntPoint) (Variables|Default|GetOriginIndex))) (Math|Conversions|ToVector(Vector2D) (Math|Conversions|ToVector2D(IntPoint) (Variables|Default|GetTargetIndex)))))
  (Utilities|FlowControl|DoOnce false
    (:Completed
      (Default|CallOnSpellAnimationHitTile self (Variables|Default|GetTargetIndex))
      (CallFunction|EventCompleteSpellAnimation))))

(fn ConstructionScript
  (|CallParentFunction))