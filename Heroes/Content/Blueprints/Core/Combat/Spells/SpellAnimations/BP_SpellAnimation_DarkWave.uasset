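; BP_SpellAnimation_DarkWave is the spell animation actor that plays the Dark Wave effect on the targeted tile.
; On play it moves to the target tile, then a timeline drives the scale and opacity of three meshes tinted in graded purple shades at construction.
; Shortly into the timeline a DoOnce reports a hit on every attacked tile, and the spell animation completes when the timeline finishes.
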(event EventEventPlaySpellAnimation
  (Transformation|SetActorLocation (.location (CallFunction|GetTileTransform (Variables|Default|GetTargetIndex))) false false)
  (bind (_direction _scale _opacity) (Timeline|Timeline_DarkWave PlayFromStart)
    (:Update
      (Transformation|SetRelativeScale3D (Variables|Default|GetAnimScale) _scale)
      (Rendering|Material|SetScalarParameterValueonMaterials (Variables|Default|GetStaticMesh) "Opacity" _opacity)
      (if (>= (Components|Timeline|GetPlaybackPosition (Variables|Default|GetTimeline_DarkWave)) 0.2)
        (Utilities|FlowControl|DoOnce false
          (:Completed
            (for _array_element (Variables|Default|GetAttackedIndexes)
              (Default|CallOnSpellAnimationHitTile self _array_element))))))
    (:Finished
      (CallFunction|EventCompleteSpellAnimation))))

(fn ConstructionScript
  (|CallParentFunction)
  (Rendering|Material|SetVectorParameterValueonMaterials (Variables|Default|GetStaticMesh) "Color" (Math|Conversions|ToVector(LinearColor) "(R=0.350000,G=0.200000,B=1.000000,A=1.000000)"))
  (Rendering|Material|SetVectorParameterValueonMaterials (Variables|Default|GetStaticMesh1) "Color" (Math|Conversions|ToVector(LinearColor) "(R=0.262500,G=0.150000,B=0.750000,A=1.000000)"))
  (Rendering|Material|SetVectorParameterValueonMaterials (Variables|Default|GetStaticMesh2) "Color" (Math|Conversions|ToVector(LinearColor) "(R=0.175000,G=0.100000,B=0.500000,A=1.000000)")))