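; Fireball spell animation actor for tile-based combat, meant to show a fireball cast from an origin tile toward a target tile.
; On play, it moves to the origin tile, yaws toward the target using grid indices as flat vectors, and spawns a system attached to its Fireball component, with no system asset specified.
; The tile-hit notification and completion calls are unwired, so neither runs.
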(event EventBeginPlay
  (|CallParentFunction) ; This node is disabled and will not be called.\nDrag off pins to build functionality.
)

(event Collision|EventActorBeginOverlap
  (params (OtherActor :type Actor%20Object%20Reference)))

(event EventTick
  (params (DeltaSeconds :type Float%20%28single-precision%29)))

(event EventEventPlaySpellAnimation
  (bind _originindex (Variables|Default|GetOriginIndex))
  (bind _originindex_2 (Variables|Default|GetOriginIndex))
  (bind _targetindex (Variables|Default|GetTargetIndex))
  (bind _transform (CallFunction|GetTileTransform _originindex_2))
  (bind _returnvalue (Math|Conversions|ToVector2D(IntPoint) _targetindex))
  (bind _returnvalue_2 (Math|Conversions|ToVector2D(IntPoint) _originindex))
  (bind _returnvalue_3 (Math|Conversions|ToVector(Vector2D) _returnvalue))
  (bind _returnvalue_4 (Math|Conversions|ToVector(Vector2D) _returnvalue_2))
  (bind _returnvalue_5 (Math|Rotator|FindLookatRotation _returnvalue_4 _returnvalue_3))
  (Transformation|SetActorLocationAndRotation (.location _transform) _returnvalue_5)
  (Niagara|SpawnSystemAttached 0 (Variables|Default|GetFireball) "None" (.location _transform) _returnvalue_5 "KeepRelativeOffset" false))

(fn ConstructionScript
  (|CallParentFunction))