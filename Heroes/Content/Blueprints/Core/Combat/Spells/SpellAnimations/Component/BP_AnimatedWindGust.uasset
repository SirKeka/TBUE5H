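; Spell animation actor that plays a wind gust visual, then destroys itself shortly after it finishes.
; Construction creates dynamic materials for two mesh slots, tinting each red with randomized brightness.
; On BeginPlay, a rate-adjustable timeline interpolates the actor from origin to target transform and drives material opacity.
; Partway through playback, it fires the shape-animation-completed event once, ahead of the timeline's end.
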(event EventBeginPlay
  (Components|Timeline|SetPlayRate (Variables|Default|GetTimeline_WindGust) (Variables|Default|GetPlayRate))
  (bind (_direction _transformalpha _opacity) (Timeline|Timeline_WindGust PlayFromStart)
    (:Update
      (Transformation|SetActorTransform (Math|Transform|Lerp(Transform) (Variables|Default|GetOriginTransform) (Variables|Default|GetTargetTransform) _transformalpha))
      (Rendering|Material|SetScalarParameterValueonMaterials (Variables|Default|GetAnimatedWindGust) "Opacity" _opacity)
      (if (>= (Components|Timeline|GetPlaybackPosition (Variables|Default|GetTimeline_WindGust)) 0.35)
        (Utilities|FlowControl|DoOnce false
          (:Completed
            (Default|CallOnShapeAnimationCompleted self)))))
    (:Finished
      (Utilities|FlowControl|Delay 0.5)
      (Actor|DestroyActor))))

(fn ConstructionScript
  (bind _returnvalue (Rendering|Material|CreateDynamicMaterialInstance (Variables|Default|GetAnimatedWindGust) 0 0 "None" :!class /Script/Engine.PrimitiveComponent))
  (Rendering|Material|SetVectorParameterValue _returnvalue "Color" (* "(R=1.000000,G=0.188843,B=0.179167,A=1.000000)" (Math|Random|RandomFloatinRange 0.8 1.5)) :!class /Script/Engine.MaterialInstanceDynamic)
  (bind _returnvalue_2 (Rendering|Material|CreateDynamicMaterialInstance (Variables|Default|GetAnimatedWindGust) 1 0 "None" :!class /Script/Engine.PrimitiveComponent))
  (Rendering|Material|SetVectorParameterValue _returnvalue_2 "Color" (* "(R=0.683333,G=0.098092,B=0.091111,A=1.000000)" (Math|Random|RandomFloatinRange 0.8 1.5)) :!class /Script/Engine.MaterialInstanceDynamic))