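; BP_SpellAnimation_Heal is the visual effect for a heal spell, played on the targeted tile.
; On play it moves to the tile, and a timeline spins and scales the mesh group while driving the opacity of six meshes.
; Once playback passes a short delay it fires the tile-hit callback a single time, then completes the spell animation when the timeline ends.
; The construction script tints the mesh pairs in three shades of blue.
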(event EventEventPlaySpellAnimation
  (bind _anim_rotationscale (Variables|Default|GetAnim_RotationScale))
  (Transformation|SetActorLocation (.location (CallFunction|GetTileTransform (Variables|Default|GetTargetIndex))) false false)
  (bind (_direction _rotation _opacity _scale) (Timeline|Timeline_Heal PlayFromStart)
    (:Update
      (Transformation|SetRelativeRotation _anim_rotationscale (Math|Rotator|MakeRotator 0.0 0.0 _rotation) false false)
      (Transformation|SetRelativeScale3D _anim_rotationscale _scale)
      (Rendering|Material|SetScalarParameterValueonMaterials (Variables|Default|GetStaticMesh) "Opacity" _opacity)
      (if (>= (Components|Timeline|GetPlaybackPosition (Variables|Default|GetTimeline_Heal)) 0.2)
        (Utilities|FlowControl|DoOnce false
          (:Completed
            (Default|CallOnSpellAnimationHitTile self (Variables|Default|GetTargetIndex))))))
    (:Finished
      (CallFunction|EventCompleteSpellAnimation))))

(fn ConstructionScript
  (|CallParentFunction)
  (Rendering|Material|SetVectorParameterValueonMaterials (Variables|Default|GetStaticMesh) "Color" (Math|Conversions|ToVector(LinearColor) "(R=0.090690,G=0.349058,B=0.500000,A=1.000000)"))
  (Rendering|Material|SetVectorParameterValueonMaterials (Variables|Default|GetStaticMesh1) "Color" (Math|Conversions|ToVector(LinearColor) "(R=0.136035,G=0.523587,B=0.750000,A=1.000000)"))
  (Rendering|Material|SetVectorParameterValueonMaterials (Variables|Default|GetStaticMesh2) "Color" (Math|Conversions|ToVector(LinearColor) "(R=0.181380,G=0.698116,B=1.000000,A=1.000000)")))