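; BP_AnimatedShape is a short-lived spell visual actor that animates a configurable mesh from an origin transform to a target transform.
; BeginPlay applies the mesh, material and color parameter, then plays a timeline at the given play rate.
; The timeline drives the transform lerp and adds a height offset curve on top of a fixed vertical lift.
; On finish it fires OnShapeAnimationCompleted and destroys itself after a brief delay.
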(event EventBeginPlay
  (bind _animatedshape (Variables|Default|GetAnimatedShape))
  (Components|StaticMesh|SetStaticMesh _animatedshape (Variables|Default|GetMesh))
  (Rendering|Material|SetMaterial _animatedshape 0 (Variables|Default|GetMaterial))
  (Rendering|Material|SetVectorParameterValueonMaterials (Variables|Default|GetAnimatedShape) "Color" (Math|Conversions|ToVector(LinearColor) (Variables|Default|GetColor)))
  (Components|Timeline|SetPlayRate (Variables|Default|GetTimeline_PlayAnimation) (Variables|Default|GetPlayRate))
  (bind (_direction _transformalpha _heghtoffset) (Timeline|Timeline_PlayAnimation PlayFromStart)
    (:Update
      (Transformation|SetActorTransform (Math|Transform|MakeTransform (+ (.Location (Math|Transform|BreakTransform (Math|Transform|Lerp(Transform) (Variables|Default|GetOriginTransform) (Variables|Default|GetTargetTransform) _transformalpha))) "0.000000,0.000000,50.000000" (Math|Vector|MakeVector 0.0 0.0 _heghtoffset)) (.Rotation (Math|Transform|BreakTransform (Math|Transform|Lerp(Transform) (Variables|Default|GetOriginTransform) (Variables|Default|GetTargetTransform) _transformalpha))) (.Scale (Math|Transform|BreakTransform (Math|Transform|Lerp(Transform) (Variables|Default|GetOriginTransform) (Variables|Default|GetTargetTransform) _transformalpha))))))
    (:Finished
      (Default|CallOnShapeAnimationCompleted self)
      (Utilities|FlowControl|Delay 0.5)
      (Actor|DestroyActor))))

(fn ConstructionScript)