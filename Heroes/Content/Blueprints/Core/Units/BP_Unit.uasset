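; Grid-based tactical combat unit actor that walks tile paths, casts spells and takes hits, with mesh and stats set from its unit type.
; A timeline moves it tile by tile, adding a jump on height changes and firing walk events.
; Spell hits change HP immediately but defer HP bar, floating number and hit/death animation until the spell animation reaches the tile.
; Hover and selection drive custom-depth stencil highlighting; combat turn hooks only print.
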(event Custom|Event_FollowPath
  (params (Path :type Array%20of%20Int%20Point%20Structures))
  ;[0 0 0] Начало движения
  (if (> (Utilities|Array|Length Path) 0)
    (Variables|Default|SetCurrentPathToFollow Path)
    (Default|CallOnUnitStartedWalking self)
    (CallFunction|ContinuetoFollowPath)))

(event Custom|ContinueToFollowPath
  (bind _timeline_unitmovement (Variables|Default|GetTimeline_UnitMovement))
  (bind _grid (Variables|Default|GetGrid))
  (bind _currentpathtofollow (Variables|Default|GetCurrentPathToFollow))
  (bind _output (Utilities|Array|Get(acopy) _currentpathtofollow))
  (bind _gridtiles (Variables|/Game/Blueprints/Core/Grid/BP_Grid.BP_Grid_C|GetGridTiles _grid))
  (bind _value (Utilities|Map|Find _gridtiles _output))
  (bind _transform (Utilities|Struct|BreakS_TileData _value))
  (bind _location (Math|Transform|BreakTransform _transform))
  ;[0 0 0] Не закончили ходить? Продолжить
  (if (> (Utilities|Array|Length (Variables|Default|GetCurrentPathToFollow)) 0)
    (CallFunction|SetAnimationState "NewEnumerator1")
    ;[0 0 0] Установите текущую плитку и следующую плитку для интерполяции
    (Variables|Default|SetPreviousTransform (Transformation|GetActorTransform))
    (Variables|Default|SetNextTransform (Math|Transform|MakeTransform _location (Math|Rotator|MakeRotator 0.0 0.0 (.Yaw (Math|Rotator|BreakRotator (Math|Rotator|FindLookatRotation (.Location (Math|Transform|BreakTransform (Variables|Default|GetPreviousTransform))) _location)))) "1.000000,1.000000,1.000000"))
    (Components|Timeline|SetPlayRate _timeline_unitmovement (/ (Components|Timeline|GetTimelineLength _timeline_unitmovement) (Variables|Default|GetMoveDurationPerTile)))
    (bind (_direction _locationalpha _rotationalpha _jump) (Timeline|Timeline_UnitMovement PlayFromStart)
      (:Update
        (Transformation|SetActorLocationAndRotation (+ (Math|Vector|Lerp(Vector) (.Location (Math|Transform|BreakTransform (Variables|Default|GetPreviousTransform))) (.Location (Math|Transform|BreakTransform (Variables|Default|GetNextTransform))) _locationalpha) (Math|Vector|MakeVector 0.0 0.0 (select (Math|Float|NearlyEqual(Float) (.Z (Class|KismetMathLibrary|BreakVector3f (.Location (Math|Transform|BreakTransform (Variables|Default|GetPreviousTransform))))) (.Z (Class|KismetMathLibrary|BreakVector3f (.Location (Math|Transform|BreakTransform (Variables|Default|GetNextTransform))))) 5.0) 0.0 _jump))) (Math|Rotator|Lerp(Rotator) (.Rotation (Math|Transform|BreakTransform (Variables|Default|GetPreviousTransform))) (.Rotation (Math|Transform|BreakTransform (Variables|Default|GetNextTransform))) _rotationalpha true)))
      (:Finished
        (Default|CallOnUnitReachedNewTile self (Utilities|Array|Get(acopy) (Variables|Default|GetCurrentPathToFollow)))
        (Utilities|Array|RemoveIndex (Variables|Default|GetCurrentPathToFollow))
        (CallFunction|ContinuetoFollowPath)))
    (else
      ;[0 0 0] Конец движения
      (CallFunction|SetAnimationState "NewEnumerator0")
      (Default|CallOnUnitFinishedWalking self))))

(event Custom|Debug_RespawnAfterFewSeconds
  (Utilities|FlowControl|Delay 2.0)
  (CallFunction|SetCurrentHP (.HP_Max (Utilities|Struct|BreakS_UnitData_Stats (Utilities|Struct|BreakS_UnitData (Variables|Default|GetUnitData)))))
  (CallFunction|SetAnimationState "NewEnumerator5")
  (Default|EventUpdateHPBar (Variables|Default|GetHPBar)))

(event EventBeginPlay
  (CallFunction|SetAnimationState "NewEnumerator0")
  (bind _output_get (Variables|Default|SetHPBar (.AsW%20HPBar (Utilities|Casting|CastToW_HPBar (UserInterface|GetUserWidgetObject (Variables|Default|GetWidget_HPBar))))))
  (Default|EventSetUnit _output_get self))

(fn ConstructionScript
  (bind _unitdata (CallFunction|GetDefaultUnitDatafromUnitType (Variables|Default|GetUnitType)))
  (CallFunction|SetUnitData _unitdata))

(fn UpdateVisualifHoveredorSelected
  (bind _skeletalmesh (Variables|Default|GetSkeletalMesh))
  (bind _skeletalmesh_2 (Variables|Default|GetSkeletalMesh))
  (if (Variables|Hovered&Selected|GetIsHovered)
    (Rendering|SetCustomDepthStencilValue (Variables|Default|GetSkeletalMesh) 1)
    (if (Variables|Hovered&Selected|GetIsSelected)
      (Rendering|SetCustomDepthStencilValue _skeletalmesh 2)
      (Rendering|SetRenderCustomDepth _skeletalmesh true)
      (else
        (Rendering|SetRenderCustomDepth (Variables|Default|GetSkeletalMesh) true)))
    (elif (Variables|Hovered&Selected|GetIsSelected)
      (Rendering|SetCustomDepthStencilValue _skeletalmesh_2 1)
      (Rendering|SetRenderCustomDepth _skeletalmesh_2 true)
      (else
        (Rendering|SetRenderCustomDepth (Variables|Default|GetSkeletalMesh) false)))))

(fn SetIsHovered
  (params (Hovered :type Boolean))
  (Variables|Hovered&Selected|SetIsHovered Hovered)
  (CallFunction|UpdateVisualifHoveredorSelected)
  (Default|CallOnUnitHoveredChanged self))

(fn SetIsSelected
  (params (Selected :type Boolean))
  (Variables|Hovered&Selected|SetIsSelected Selected)
  (CallFunction|UpdateVisualifHoveredorSelected)
  (Default|CallOnUnitSelectedChanged self))

(fn SetUnitData
  (params (Data :type S%20Unit%20Data%20Structure%20%28by%20ref%29))
  (bind _skeletalmesh (Variables|Default|GetSkeletalMesh))
  (bind _output_get (Variables|Default|SetUnitData Data))
  (Components|SkinnedMesh|SetSkinnedAssetandUpdate _skeletalmesh (.Mesh (Utilities|Struct|BreakS_UnitData_Assets (.Assets (Utilities|Struct|BreakS_UnitData _output_get)))) true)
  (Class|SkeletalMeshComponent|SetAnimClass _skeletalmesh (.AnimBP (Utilities|Struct|BreakS_UnitData_Assets (.Assets (Utilities|Struct|BreakS_UnitData _output_get)))))
  (CallFunction|UpdateVisualifHoveredorSelected))

(fn SetAnimationState
  (params (State :type E_UnitAnimationState%20Enum :default "NewEnumerator0"))
  (Class|BPIUnitAnimation|SetUnitAnimationState(Message) (Components|SkeletalMesh|GetAnimInstance (Variables|Default|GetSkeletalMesh)) State))

(fn SetGrid
  (params (Grid :type BP%20Grid%20Object%20Reference))
  (bind _collision_lineofsight (Variables|Default|GetCollision_LineOfSight))
  (Variables|Default|SetGrid Grid)
  (Components|StaticMesh|SetStaticMesh _collision_lineofsight (.Mesh (Utilities|Struct|BreakS_GridShapeData (Default|GetCurrentShape (Variables|Default|GetGrid)))))
  (Transformation|SetAbsolute _collision_lineofsight false true true)
  (Transformation|SetWorldScale3D _collision_lineofsight (Math|Vector|MakeVector (.x (/ (Variables|/Game/Blueprints/Core/Grid/BP_Grid.BP_Grid_C|GetGridTileSize (Variables|Default|GetGrid)) (.MeshSize (Utilities|Struct|BreakS_GridShapeData (Default|GetCurrentShape (Variables|Default|GetGrid)))))) (.y (/ (Variables|/Game/Blueprints/Core/Grid/BP_Grid.BP_Grid_C|GetGridTileSize (Variables|Default|GetGrid)) (.MeshSize (Utilities|Struct|BreakS_GridShapeData (Default|GetCurrentShape (Variables|Default|GetGrid)))))) (.z (Transformation|GetWorldScale (Variables|Default|GetCollision_LineOfSight))))))

(fn UnitCastSpell
  (params (TargetIndex :type Int%20Point%20Structure))
  (bind _returnvalue (Transformation|GetActorLocation))
  (bind _grid (Variables|Default|GetGrid))
  (bind (_x _y) (Math|Vector|BreakVector _returnvalue))
  (bind _gridtiles (Variables|/Game/Blueprints/Core/Grid/BP_Grid.BP_Grid_C|GetGridTiles _grid))
  (bind _value (Utilities|Map|Find _gridtiles TargetIndex))
  (bind _transform (Utilities|Struct|BreakS_TileData _value))
  (bind (_x_2 _y_2) (Math|Vector|BreakVector (.location _transform)))
  (Transformation|SetActorRotation (Math|Rotator|FindLookatRotation (Math|Vector|MakeVector _x _y 0.0) (Math|Vector|MakeVector _x_2 _y_2 0.0)))
  (CallFunction|SetAnimationState "NewEnumerator2"))

(fn SetCurrentHP
  (params (HP :type Integer))
  (bind _structout (Utilities|Struct|SetmembersinS_UnitData_Stats (Utilities|Struct|BreakS_UnitData (Variables|Default|GetUnitData)) (Math|Integer|Clamp(Integer) HP 0 (.HP_Max (Utilities|Struct|BreakS_UnitData_Stats (Utilities|Struct|BreakS_UnitData (Variables|Default|GetUnitData)))))))
  (Utilities|Struct|SetmembersinS_UnitData (Variables|Default|GetUnitData) _structout))

(fn ModifierCurrentHP
  (params (Modifier :type Integer))
  (CallFunction|SetCurrentHP (+ Modifier (.HP_Current (Utilities|Struct|BreakS_UnitData_Stats (Utilities|Struct|BreakS_UnitData (Variables|Default|GetUnitData)))))))

(fn UnitHitbySpell
  (params (SpellImpactReal :type S%20Spell%20Data%20Impact%20Real%20Structure) (SpellAnimation :type BP%20Spell%20Animation%20Object%20Reference))
  (bind _modifier_hp (Utilities|Struct|BreakS_SpellData_ImpactReal SpellImpactReal))
  (Utilities|Map|Add (Variables|Default|GetIncomingSpellImpact) SpellAnimation SpellImpactReal)
  (EventDispatchers|BindEventtoOnSpellAnimationHitTile SpellAnimation (EventDispatchers|CreateEvent :!event OnSpellAnimationHitTile))
  (if (!= _modifier_hp 0) ; HP Изменяется?
    (CallFunction|ModifierCurrentHP _modifier_hp)))

(fn OnSpellAnimationHitTile
  (params (SpellAnimation :type BP%20Spell%20Animation%20Object%20Reference) (Index :type Int%20Point%20Structure))
  (bind _incomingspellimpact (Variables|Default|GetIncomingSpellImpact))
  (bind (_value _returnvalue) (Utilities|Map|Find _incomingspellimpact SpellAnimation))
  ;[0 0 0] Мы обрабатываем это заклинание?
  (if (Class|KismetMathLibrary|EqualIntPointIntPoint (Variables|Default|GetIndex) Index) ; Это моя плитка?
    (if _returnvalue ; Мне все еще нужно обработать это заклинание?
      (LocalVariables|SetSpellImpactReal _value)
      (Utilities|Map|Remove (Variables|Default|GetIncomingSpellImpact) SpellAnimation)
      (Default|EventUpdateHPBar (Variables|Default|GetHPBar))
      (Game|SpawnActorfromClass "/Game/Blueprints/Core/Units/Widgets/BP_AnimatedNumber.BP_AnimatedNumber_C" (Math|Transform|MakeTransform (Transformation|GetActorLocation) "0, 0, 0" "1.000000,1.000000,1.000000") "Undefined" 0 (Utilities|Struct|BreakS_SpellData_ImpactReal (LocalVariables|GetSpellImpactReal)) 0)
      ;[0 0 0] Если это наносящее урон заклинание, мы либо просим юнита воспроизвести анимацию удара, либо анимацию смерти, в зависимости от того, жив он или нет.
      (if (< (Utilities|Struct|BreakS_SpellData_ImpactReal (LocalVariables|GetSpellImpactReal)) 0) ; Повредил единицу?
        (if (== (.HP_Current (Utilities|Struct|BreakS_UnitData_Stats (Utilities|Struct|BreakS_UnitData (Variables|Default|GetUnitData)))) 0) ; Он мертв?
          (if (Utilities|Enum|NotEqual(Enum) (CallFunction|GetAnimationState) "NewEnumerator4")
            (CallFunction|SetAnimationState "NewEnumerator4"))
          (else
            (CallFunction|SetAnimationState "NewEnumerator3")))))))

(fn GetAnimationState
  (bind _state (Class|BPIUnitAnimation|GetUnitAnimationState(Message) (Components|SkeletalMesh|GetAnimInstance (Variables|Default|GetSkeletalMesh))))
  (return _state))

(fn SetTeamIndex
  (params (Index :type Integer))
  (Variables|Default|SetTeamIndex Index)
  (Class|ProgressBar|SetFillColorandOpacity (Variables|/Game/Blueprints/Core/Units/Widgets/W_HPBar.W_HPBar_C|GetProgressBar_HP (Variables|Default|GetHPBar)) (CallFunction|GetTeamColor (Variables|Default|GetTeamIndex))))

(fn CombatStarted
  (Development|PrintString "Я в бою"))

(fn TurnStarted
  (Development|PrintString "Это мой ход"))

(fn TurnEnded
  (Development|PrintString "Время спать!"))

(fn CombatEnded
  (Development|PrintString "Каникулы!"))