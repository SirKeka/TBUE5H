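; Manager for overworld unit groups, keeping units in a map keyed by group ID with an encounter flag per group.
; Adding a unit moves it from its previous group and binds its events; destroyed units are removed and emptied groups deleted.
; Hovering one member mirrors the state to the group, and walking makes the others follow in a chain.
; Both propagations temporarily unbind each member's event to avoid re-entrant callbacks.
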(event EventBeginPlay)

(event Collision|EventActorBeginOverlap
  (params (OtherActor :type Actor%20Object%20Reference)))

(event EventTick
  (params (DeltaSeconds :type Float%20%28single-precision%29)))

(fn ConstructionScript)

(fn AddUnitonGroup
  (params (Unit :type BP%20Unit%20Object%20Reference) (GroupID :type Integer))
  (if (!= (Variables|/Game/Blueprints/Core/Units/BP_Unit.BP_Unit_C|GetOverworldGroup_ID Unit) GroupID)
    (CallFunction|RemoveUnitfromCurrentGroup Unit)
    (if (!= GroupID -999)
      (bind _output_get (LocalVariables|SetGroup (.Value (Utilities|Map|Find (Variables|Default|GetUnitGroups) GroupID))))
      (Utilities|Array|Add (Utilities|Struct|BreakS_OverworldUnitGroup _output_get) Unit)
      (Utilities|Map|Add (Variables|Default|GetUnitGroups) GroupID (LocalVariables|GetGroup))
      (Variables|/Game/Blueprints/Core/Units/BP_Unit.BP_Unit_C|SetOverworldGroup_ID Unit GroupID)
      ;[1 1 1] Если мы не хотим удалять юнитов из группы после смерти для будущего их воскрешения, то отключить
      (Game|BindEventtoOnDestroyed Unit (EventDispatchers|CreateEvent :!event OnUnitDestroyed))
      (EventDispatchers|BindEventtoOnUnitHoveredChanged Unit (EventDispatchers|CreateEvent :!event OnUnitHoveredChanged))
      (EventDispatchers|BindEventtoOnUnitStartedWalkinginOverworld Unit (EventDispatchers|CreateEvent :!event OnUnitStartedWalkinginOverworld)))))

(fn RemoveUnitfromCurrentGroup
  (params (Unit :type BP%20Unit%20Object%20Reference))
  (if (!= (Variables|/Game/Blueprints/Core/Units/BP_Unit.BP_Unit_C|GetOverworldGroup_ID Unit) -999)
    (bind _output_get (LocalVariables|SetGroup (.Value (Utilities|Map|Find (Variables|Default|GetUnitGroups) (Variables|/Game/Blueprints/Core/Units/BP_Unit.BP_Unit_C|GetOverworldGroup_ID Unit)))))
    (Utilities|Array|RemoveItem (Utilities|Struct|BreakS_OverworldUnitGroup _output_get) Unit)
    (if (> (Utilities|Array|Length (Utilities|Struct|BreakS_OverworldUnitGroup _output_get)) 0)
      (Utilities|Map|Add (Variables|Default|GetUnitGroups) (Variables|/Game/Blueprints/Core/Units/BP_Unit.BP_Unit_C|GetOverworldGroup_ID Unit) (LocalVariables|GetGroup))
      (else
        (Utilities|Map|Remove (Variables|Default|GetUnitGroups) (Variables|/Game/Blueprints/Core/Units/BP_Unit.BP_Unit_C|GetOverworldGroup_ID Unit))))
    (Variables|/Game/Blueprints/Core/Units/BP_Unit.BP_Unit_C|SetOverworldGroup_ID Unit -999)
    (EventDispatchers|UnbindEventfromOnUnitHoveredChanged Unit (EventDispatchers|CreateEvent :!event OnUnitHoveredChanged))
    (EventDispatchers|UnbindEventfromOnUnitStartedWalkinginOverworld Unit (EventDispatchers|CreateEvent :!event OnUnitStartedWalkinginOverworld))))

(fn OnUnitDestroyed
  (params (DestroyedActor :type Actor%20Object%20Reference))
  (Utilities|Casting|CastToBP_Unit DestroyedActor)
  (CallFunction|RemoveUnitfromCurrentGroup))

(fn OnUnitHoveredChanged
  (params (Unit :type BP%20Unit%20Object%20Reference))
  (bind _overworldgroup_id (Variables|/Game/Blueprints/Core/Units/BP_Unit.BP_Unit_C|GetOverworldGroup_ID Unit))
  (bind _unitgroups (Variables|Default|GetUnitGroups))
  (bind (_value _returnvalue) (Utilities|Map|Find _unitgroups _overworldgroup_id))
  (if _returnvalue
    (bind _output_get (LocalVariables|SetG _value))
    (for _array_element (Utilities|Struct|BreakS_OverworldUnitGroup _output_get)
      (bind _output_get_2 (LocalVariables|SetU _array_element))
      (if (!= _output_get_2 Unit)
        (EventDispatchers|UnbindEventfromOnUnitHoveredChanged (LocalVariables|GetU) (EventDispatchers|CreateEvent :!event OnUnitHoveredChanged))
        (Default|SetIsHovered (LocalVariables|GetU) (Variables|/Game/Blueprints/Core/Units/BP_Unit.BP_Unit_C|GetIsHovered Unit))
        (EventDispatchers|BindEventtoOnUnitHoveredChanged (LocalVariables|GetU) (EventDispatchers|CreateEvent :!event OnUnitHoveredChanged))))))

(fn OnUnitStartedWalkinginOverworld
  (params (Unit :type BP%20Unit%20Object%20Reference))
  (LocalVariables|SetPreviousUnitInChain Unit)
  (for _array_element (Utilities|Struct|BreakS_OverworldUnitGroup (.Value (Utilities|Map|Find (Variables|Default|GetUnitGroups) (Variables|/Game/Blueprints/Core/Units/BP_Unit.BP_Unit_C|GetOverworldGroup_ID Unit))))
    (bind _output_get (LocalVariables|SetUn _array_element))
    (if (!= _output_get Unit)
      (EventDispatchers|UnbindEventfromOnUnitStartedWalkinginOverworld (LocalVariables|GetUn) (EventDispatchers|CreateEvent :!event OnUnitStartedWalkinginOverworld))
      (Default|EventMoveUnitinOverworld (LocalVariables|GetUn) "0, 0, 0" (LocalVariables|GetPreviousUnitInChain))
      (LocalVariables|SetPreviousUnitInChain (LocalVariables|GetUn))
      (EventDispatchers|BindEventtoOnUnitStartedWalkinginOverworld (LocalVariables|GetUn) (EventDispatchers|CreateEvent :!event OnUnitStartedWalkinginOverworld)))))

(fn SetGroupIsEncounter
  (params (IsEncounter :type Boolean) (GroupID :type Integer))
  (bind _unitgroups (Variables|Default|GetUnitGroups))
  (bind (_value _returnvalue) (Utilities|Map|Find _unitgroups GroupID))
  (if _returnvalue
    (bind _output_get (LocalVariables|SetGr _value))
    (if (!= (Utilities|Struct|BreakS_OverworldUnitGroup _output_get) IsEncounter)
      (Utilities|Struct|SetmembersinS_OverworldUnitGroup (LocalVariables|GetGr) IsEncounter)
      (Utilities|Map|Add (Variables|Default|GetUnitGroups) GroupID (LocalVariables|GetGr)))))