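; Ranger unit AI that varies its movement logic by turn parity and whether it has cast a damaging spell this turn.
; Counts turns from combat start and clears the damage flag each turn, extending the parent's turn flow.
; Casting a spell with a negative minimum HP modifier sets the flag.
; Even turns without damage use one movement mode; all other cases use another.
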(event EventBeginPlay
  (|CallParentFunction) ; This node is disabled and will not be called.\nDrag off pins to build functionality.
)

(event Collision|EventActorBeginOverlap
  (params (OtherActor :type Actor%20Object%20Reference)))

(event EventTick
  (params (DeltaSeconds :type Float%20%28single-precision%29)))

(event EventCastSpel
  (bind _spell_data (CallFunction|GetSpellDatafromSpell (Utilities|Struct|BreakS_UnitAI_SpellCastingData (Variables|Default|GetAI_SpellCasting))))
  (Variables|Default|SetDamageAnUnitThisTurn (or (Variables|Default|GetDamageAnUnitThisTurn) (< (.X (Utilities|Struct|BreakIntPoint (Utilities|Struct|BreakS_SpellData_Impact (Utilities|Struct|BreakS_SpellData _spell_data)))) 0)))
  (|CallParentFunction))

(fn ConstructionScript
  (|CallParentFunction))

(fn AIPlayTurn
  (Math|Integer|IncrementInt (Variables|Default|GetTurnCount)
    (:%20%20
      (Variables|Default|SetDamageAnUnitThisTurn false)
      (|CallParentFunction))))

(fn GetUnitMovementLogic
  (return (select (and (CallFunction|IsIntEven (Variables|Default|GetTurnCount)) (not (Variables|Default|GetDamageAnUnitThisTurn))) "NewEnumerator0" "NewEnumerator2")))

(fn AICombatStarted
  (Variables|Default|SetTurnCount 0)
  (|CallParentFunction))